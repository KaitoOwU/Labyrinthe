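; BP_IJRGenerator is a spawner that releases a rapid burst of BP_IndianaJonesRocks actors at its own transform.
; SetIJRTimer starts a looping function-name timer that calls GenerateRock several times per second.
; GenerateRock spawns one rock per call, counts it, and clears the timer once the count reaches twenty.
; Nothing in the file calls SetIJRTimer or resets the count.
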(fn `GenerateRock`
  (`|SpawnActorFromClass` "/Game/Le_Labyrinthe/Blueprints/BP_IndianaJonesRocks.BP_IndianaJonesRocks_C" (`self.GetTransform`) "Undefined" "OverrideRootScale" null null)
  (bind _output_get (set `self.AmountOfRock` (+ (`self.AmountOfRock`) 1)))
  (if (>= _output_get 20)
    (`KismetSystemLibrary.K2_ClearAndInvalidateTimerHandle` (`self.Timer`))))

(fn `SetIJRTimer`
  (bind _returnvalue (`KismetSystemLibrary.K2_SetTimer` null "GenerateRock" 0.1 true))
  (set `self.Timer` _returnvalue))

(fn `UserConstructionScript`)